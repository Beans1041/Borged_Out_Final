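; BP_car_fly_black1 is a flying car actor in CyberCity with purely procedural idle animation.
; Every tick it spins two FlashRot components in opposite yaw directions by a fixed per-frame step, so their speed depends on frame rate.
; It also sets the root's roll and pitch from game-time sine waves at different frequencies for a gentle hovering sway, holding yaw at zero.
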(event EventTick
  (params (DeltaSeconds :type Float%20%28single-precision%29))
  (bind _returnvalue (Utilities|Time|GetGameTimeinSeconds))
  (Transformation|AddRelativeRotation (Variables|Default|GetSM_car_fly_flash_rot) "0.000000,6.000000,0.000000" false false)
  (Transformation|AddRelativeRotation (Variables|Default|GetSM_car_fly_flash_rot1) "0.000000,-6.000000,0.000000" false false)
  (Transformation|SetRelativeRotation (Variables|Default|GetDefaultSceneRoot) (Math|Rotator|MakeRotator (* (Math|Trig|Sin(Degrees) (* _returnvalue 5e+01)) 2.0) (* (Math|Trig|Sin(Degrees) (* _returnvalue 3e+01)) 2.0) 0.0) false false))

(fn ConstructionScript)