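; BP_traffic_light is a street traffic light prop for the CyberCity environment with configurable light components.
; The construction script sets the visibility of four SMTrafficLightLighter components from the Unhide0 to Unhide3 variables, without propagating to children.
; The event graph holds only disabled placeholder events, so it runs no gameplay logic or signal cycling.
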(event EventBeginPlay)

(event Collision|EventActorBeginOverlap
  (params (OtherActor :type Actor%20Object%20Reference)))

(event EventTick
  (params (DeltaSeconds :type Float%20%28single-precision%29)))

(fn ConstructionScript
  (Rendering|SetVisibility (Variables|Default|GetSM_traffic_light_lighter0) (Variables|CCControl|GetUnhide0) false)
  (Rendering|SetVisibility (Variables|Default|GetSM_traffic_light_lighter1) (Variables|CCControl|GetUnhide1) false)
  (Rendering|SetVisibility (Variables|Default|GetSM_traffic_light_lighter2) (Variables|CCControl|GetUnhide2) false)
  (Rendering|SetVisibility (Variables|Default|GetSM_traffic_light_lighter3) (Variables|CCControl|GetUnhide3) false))