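; BP_robot_7 is a robot actor in the CyberCity content that gives its SMRobot3 mesh a continuous idle wobble.
; Each tick it sets the mesh's relative rotation from sine waves of game time, with separate frequency and power variables for roll and pitch.
; Yaw is held at zero and the construction script is empty.
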(event EventTick
  (params (DeltaSeconds :type Float%20%28single-precision%29))
  (bind _returnvalue (Utilities|Time|GetGameTimeinSeconds))
  (Transformation|SetRelativeRotation (Variables|Default|GetSM_robot_3) (Math|Rotator|MakeRotator (* (Math|Trig|Sin(Degrees) (* _returnvalue (Variables|Default|GetRollFrequency))) (Variables|Default|GetRollPower)) (* (Math|Trig|Sin(Degrees) (* _returnvalue (Variables|Default|GetPitchFrequency))) (Variables|Default|GetPitchPower)) 0.0) false false))

(fn ConstructionScript)